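; BP_Camera is the side-scroller's level camera, which follows the player vertically and also handles death by falling.
; On BeginPlay it caches the 2DSideScrollerCharacter and becomes the player controller's view target.
; Each tick it matches the camera's Z to the pawn's, keeping X and Y unchanged.
; Once the pawn drops to a fixed height threshold, it stops ticking, flags the character dead and calls UnloadStreamLevel on the current level name.
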(event `self.ReceiveBeginPlay`
  (bind _as2dside_scroller_character (cast `/Game/2DSideScrollerBP/Blueprints/2DSideScrollerCharacter` (`GameplayStatics.GetPlayerCharacter` 0)))
  (`PlayerController.SetViewTargetWithBlend` (`GameplayStatics.GetPlayerController` 0) self 0.0 "VTBlend_Linear" 0.0 false))

(event `self.ReceiveTick`
  (params (DeltaSeconds :type "Float (single-precision)"))
  (bind _camera (`self.Camera`))
  (bind (_returnvalue_x _returnvalue_y _returnvalue_z) (`KismetMathLibrary.BreakVector` (`self.K2_GetActorLocation` (`GameplayStatics.GetPlayerPawn` 0))))
  (bind (_returnvalue_x_2 _returnvalue_y_2) (`KismetMathLibrary.BreakVector` (`SceneComponent.K2_GetComponentLocation` _camera)))
  ;[1 1 1] 相机位置
  (if (<= _returnvalue_z 150.0)
    (`/Engine/EditorBlueprintResources/StandardMacros.DoOnce` false
      (:`Completed`
        (`self.SetActorTickEnabled` false)
        (bind _returnvalue (`GameplayStatics.GetCurrentLevelName` true))
        (if (not (`/Game/2DSideScrollerBP/Blueprints/2DSideScrollerCharacter.If Dead` (stale `self.ReceiveBeginPlay` _as2dside_scroller_character)))
          (set `/Game/2DSideScrollerBP/Blueprints/2DSideScrollerCharacter.If Dead` true (stale `self.ReceiveBeginPlay` _as2dside_scroller_character)))
        (`GameplayStatics.UnloadStreamLevel` (`KismetStringLibrary.Conv_StringToName` _returnvalue))))
    (else
      (`SceneComponent.K2_SetWorldLocation` _camera (`KismetMathLibrary.MakeVector` _returnvalue_x_2 _returnvalue_y_2 _returnvalue_z) false false))))

(fn `UserConstructionScript`)