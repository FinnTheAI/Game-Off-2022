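; Shared function library that handles menu button focus styling and starts background music.
; CheckFocus and CheckFocus_Claws make a hovered button take keyboard focus with a mouse style, otherwise applying selected or normal styles by keyboard focus.
; PlayMusic creates either the UI or gameplay track as a 2D sound, fades it in, and returns both audio references.
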(fn `CheckFocus`
  (params (NewParam :type "Button Object Reference"))
  (locals (KeyNotStyle :type "ButtonStyle Structure" :default (struct :`Normal` (struct :`ImageSize` (32.0 32.0) :`Margin` (struct) :`TintColor` (struct :`SpecifiedColor` (struct :`R` 1.0 :`G` 0.590619 :`B` 0.162029 :`A` 1.0) :`ColorUseRule` "UseColor_Specified") :`OutlineSettings` (struct :`CornerRadii` (struct :`X` 60.0 :`Y` 60.0 :`Z` 60.0 :`W` 60.0) :`Color` (struct :`SpecifiedColor` (struct) :`ColorUseRule` "UseColor_Specified") :`RoundingType` "HalfHeightRadius") :`UVRegion` (struct :`Min` (0.0 0.0) :`Max` (0.0 0.0)) :`DrawAs` "RoundedBox" :`Tiling` "NoTile" :`Mirroring` "NoMirror" :`ImageType` "NoImage") :`Hovered` (struct :`ImageSize` (32.0 32.0) :`Margin` (struct) :`TintColor` (struct :`SpecifiedColor` (struct :`R` 0.83077 :`G` 0.198069 :`A` 1.0) :`ColorUseRule` "UseColor_Specified") :`OutlineSettings` (struct :`CornerRadii` (struct :`X` 60.0 :`Y` 60.0 :`Z` 60.0 :`W` 60.0) :`Color` (struct :`SpecifiedColor` (struct) :`ColorUseRule` "UseColor_Specified") :`RoundingType` "HalfHeightRadius") :`UVRegion` (struct :`Min` (0.0 0.0) :`Max` (0.0 0.0)) :`DrawAs` "RoundedBox" :`Tiling` "NoTile" :`Mirroring` "NoMirror" :`ImageType` "NoImage") :`Pressed` (struct :`ImageSize` (32.0 32.0) :`Margin` (struct) :`TintColor` (struct :`SpecifiedColor` (struct :`R` 0.62396 :`G` 0.014444 :`B` 0.08022 :`A` 1.0) :`ColorUseRule` "UseColor_Specified") :`OutlineSettings` (struct :`CornerRadii` (struct :`X` 60.0 :`Y` 60.0 :`Z` 60.0 :`W` 60.0) :`Color` (struct :`SpecifiedColor` (struct) :`ColorUseRule` "UseColor_Specified") :`RoundingType` "HalfHeightRadius") :`UVRegion` (struct :`Min` (0.0 0.0) :`Max` (0.0 0.0)) :`DrawAs` "RoundedBox" :`Tiling` "NoTile" :`Mirroring` "NoMirror" :`ImageType` "NoImage") :`Disabled` (struct :`ImageSize` (0.0 0.0) :`Margin` (struct) :`TintColor` (struct :`SpecifiedColor` (struct :`R` 1.0 :`G` 1.0 :`B` 1.0 :`A` 1.0) :`ColorUseRule` "UseColor_Specified") :`OutlineSettings` (struct :`CornerRadii` (struct :`W` 1.0) :`Color` (struct :`SpecifiedColor` (struct) :`ColorUseRule` "UseColor_Specified") :`RoundingType` "HalfHeightRadius") :`UVRegion` (struct :`Min` (0.0 0.0) :`Max` (0.0 0.0)) :`DrawAs` "NoDrawType" :`Tiling` "NoTile" :`Mirroring` "NoMirror" :`ImageType` "NoImage") :`NormalForeground` (struct :`SpecifiedColor` (struct :`R` 1.0 :`B` 1.0 :`A` 1.0) :`ColorUseRule` "UseColor_Foreground") :`HoveredForeground` (struct :`SpecifiedColor` (struct :`R` 1.0 :`B` 1.0 :`A` 1.0) :`ColorUseRule` "UseColor_Foreground") :`PressedForeground` (struct :`SpecifiedColor` (struct :`R` 1.0 :`B` 1.0 :`A` 1.0) :`ColorUseRule` "UseColor_Foreground") :`DisabledForeground` (struct :`SpecifiedColor` (struct :`R` 1.0 :`B` 1.0 :`A` 1.0) :`ColorUseRule` "UseColor_Foreground") :`NormalPadding` (struct) :`PressedPadding` (struct) :`PressedSlateSound` (struct) :`HoveredSlateSound` (struct))) (MouseStyle_new :type "ButtonStyle Structure" :default (struct :`Normal` (struct :`ImageSize` (32.0 32.0) :`Margin` (struct) :`TintColor` (struct :`SpecifiedColor` (struct :`R` 1.0 :`G` 0.590619 :`B` 0.162029 :`A` 1.0) :`ColorUseRule` "UseColor_Specified") :`OutlineSettings` (struct :`CornerRadii` (struct :`X` 60.0 :`Y` 60.0 :`Z` 60.0 :`W` 60.0) :`Color` (struct :`SpecifiedColor` (struct) :`ColorUseRule` "UseColor_Specified") :`RoundingType` "HalfHeightRadius") :`UVRegion` (struct :`Min` (0.0 0.0) :`Max` (0.0 0.0)) :`DrawAs` "RoundedBox" :`Tiling` "NoTile" :`Mirroring` "NoMirror" :`ImageType` "NoImage") :`Hovered` (struct :`ImageSize` (32.0 32.0) :`Margin` (struct) :`TintColor` (struct :`SpecifiedColor` (struct :`R` 0.83077 :`G` 0.198069 :`A` 1.0) :`ColorUseRule` "UseColor_Specified") :`OutlineSettings` (struct :`CornerRadii` (struct :`X` 60.0 :`Y` 60.0 :`Z` 60.0 :`W` 60.0) :`Color` (struct :`SpecifiedColor` (struct) :`ColorUseRule` "UseColor_Specified") :`RoundingType` "HalfHeightRadius") :`UVRegion` (struct :`Min` (0.0 0.0) :`Max` (0.0 0.0)) :`DrawAs` "RoundedBox" :`Tiling` "NoTile" :`Mirroring` "NoMirror" :`ImageType` "NoImage") :`Pressed` (struct :`ImageSize` (32.0 32.0) :`Margin` (struct) :`TintColor` (struct :`SpecifiedColor` (struct :`R` 0.62396 :`G` 0.014444 :`B` 0.08022 :`A` 1.0) :`ColorUseRule` "UseColor_Specified") :`OutlineSettings` (struct :`CornerRadii` (struct :`X` 60.0 :`Y` 60.0 :`Z` 60.0 :`W` 60.0) :`Color` (struct :`SpecifiedColor` (struct) :`ColorUseRule` "UseColor_Specified") :`RoundingType` "HalfHeightRadius") :`UVRegion` (struct :`Min` (0.0 0.0) :`Max` (0.0 0.0)) :`DrawAs` "RoundedBox" :`Tiling` "NoTile" :`Mirroring` "NoMirror" :`ImageType` "NoImage") :`Disabled` (struct :`ImageSize` (0.0 0.0) :`Margin` (struct) :`TintColor` (struct :`SpecifiedColor` (struct :`R` 1.0 :`G` 1.0 :`B` 1.0 :`A` 1.0) :`ColorUseRule` "UseColor_Specified") :`OutlineSettings` (struct :`CornerRadii` (struct :`W` 1.0) :`Color` (struct :`SpecifiedColor` (struct) :`ColorUseRule` "UseColor_Specified") :`RoundingType` "HalfHeightRadius") :`UVRegion` (struct :`Min` (0.0 0.0) :`Max` (0.0 0.0)) :`DrawAs` "NoDrawType" :`Tiling` "NoTile" :`Mirroring` "NoMirror" :`ImageType` "NoImage") :`NormalForeground` (struct :`SpecifiedColor` (struct :`R` 1.0 :`B` 1.0 :`A` 1.0) :`ColorUseRule` "UseColor_Foreground") :`HoveredForeground` (struct :`SpecifiedColor` (struct :`R` 1.0 :`B` 1.0 :`A` 1.0) :`ColorUseRule` "UseColor_Foreground") :`PressedForeground` (struct :`SpecifiedColor` (struct :`R` 1.0 :`B` 1.0 :`A` 1.0) :`ColorUseRule` "UseColor_Foreground") :`DisabledForeground` (struct :`SpecifiedColor` (struct :`R` 1.0 :`B` 1.0 :`A` 1.0) :`ColorUseRule` "UseColor_Foreground") :`NormalPadding` (struct) :`PressedPadding` (struct) :`PressedSlateSound` (struct) :`HoveredSlateSound` (struct))) (KeySelected_new :type "ButtonStyle Structure" :default (struct :`Normal` (struct :`ImageSize` (32.0 32.0) :`Margin` (struct) :`TintColor` (struct :`SpecifiedColor` (struct :`R` 0.83077 :`G` 0.198069 :`A` 1.0) :`ColorUseRule` "UseColor_Specified") :`OutlineSettings` (struct :`CornerRadii` (struct :`X` 60.0 :`Y` 60.0 :`Z` 60.0 :`W` 60.0) :`Color` (struct :`SpecifiedColor` (struct) :`ColorUseRule` "UseColor_Specified") :`RoundingType` "HalfHeightRadius") :`UVRegion` (struct :`Min` (0.0 0.0) :`Max` (0.0 0.0)) :`DrawAs` "RoundedBox" :`Tiling` "NoTile" :`Mirroring` "NoMirror" :`ImageType` "NoImage") :`Hovered` (struct :`ImageSize` (32.0 32.0) :`Margin` (struct) :`TintColor` (struct :`SpecifiedColor` (struct :`R` 0.83077 :`G` 0.198069 :`A` 1.0) :`ColorUseRule` "UseColor_Specified") :`OutlineSettings` (struct :`CornerRadii` (struct :`X` 60.0 :`Y` 60.0 :`Z` 60.0 :`W` 60.0) :`Color` (struct :`SpecifiedColor` (struct) :`ColorUseRule` "UseColor_Specified") :`RoundingType` "HalfHeightRadius") :`UVRegion` (struct :`Min` (0.0 0.0) :`Max` (0.0 0.0)) :`DrawAs` "RoundedBox" :`Tiling` "NoTile" :`Mirroring` "NoMirror" :`ImageType` "NoImage") :`Pressed` (struct :`ImageSize` (32.0 32.0) :`Margin` (struct) :`TintColor` (struct :`SpecifiedColor` (struct :`R` 0.62396 :`G` 0.014444 :`B` 0.08022 :`A` 1.0) :`ColorUseRule` "UseColor_Specified") :`OutlineSettings` (struct :`CornerRadii` (struct :`X` 60.0 :`Y` 60.0 :`Z` 60.0 :`W` 60.0) :`Color` (struct :`SpecifiedColor` (struct) :`ColorUseRule` "UseColor_Specified") :`RoundingType` "HalfHeightRadius") :`UVRegion` (struct :`Min` (0.0 0.0) :`Max` (0.0 0.0)) :`DrawAs` "RoundedBox" :`Tiling` "NoTile" :`Mirroring` "NoMirror" :`ImageType` "NoImage") :`Disabled` (struct :`ImageSize` (0.0 0.0) :`Margin` (struct) :`TintColor` (struct :`SpecifiedColor` (struct :`R` 1.0 :`G` 1.0 :`B` 1.0 :`A` 1.0) :`ColorUseRule` "UseColor_Specified") :`OutlineSettings` (struct :`CornerRadii` (struct :`W` 1.0) :`Color` (struct :`SpecifiedColor` (struct) :`ColorUseRule` "UseColor_Specified") :`RoundingType` "HalfHeightRadius") :`UVRegion` (struct :`Min` (0.0 0.0) :`Max` (0.0 0.0)) :`DrawAs` "NoDrawType" :`Tiling` "NoTile" :`Mirroring` "NoMirror" :`ImageType` "NoImage") :`NormalForeground` (struct :`SpecifiedColor` (struct :`R` 1.0 :`B` 1.0 :`A` 1.0) :`ColorUseRule` "UseColor_Foreground") :`HoveredForeground` (struct :`SpecifiedColor` (struct :`R` 1.0 :`B` 1.0 :`A` 1.0) :`ColorUseRule` "UseColor_Foreground") :`PressedForeground` (struct :`SpecifiedColor` (struct :`R` 1.0 :`B` 1.0 :`A` 1.0) :`ColorUseRule` "UseColor_Foreground") :`DisabledForeground` (struct :`SpecifiedColor` (struct :`R` 1.0 :`B` 1.0 :`A` 1.0) :`ColorUseRule` "UseColor_Foreground") :`NormalPadding` (struct) :`PressedPadding` (struct) :`PressedSlateSound` (struct) :`HoveredSlateSound` (struct))))
  (if (`Widget.IsHovered` NewParam)
    (`Widget.SetKeyboardFocus` NewParam)
    (`Button.SetStyle` NewParam (`local.MouseStyle_new`))
    (else
      (`Button.SetStyle` NewParam (select `bool` (`Widget.HasKeyboardFocus` NewParam) :`false` (`local.KeyNotStyle`) :`true` (`local.KeySelected_new`))))))

(fn `CheckFocus_Claws`
  (params (NewParam :type "Button Object Reference"))
  (locals (KeyNotStyle :type "ButtonStyle Structure" :default (struct :`Normal` (struct :`ImageSize` (32.0 32.0) :`Margin` (struct) :`TintColor` (struct :`SpecifiedColor` (struct :`R` 1.0 :`G` 0.590619 :`B` 0.162029) :`ColorUseRule` "UseColor_Specified") :`OutlineSettings` (struct :`CornerRadii` (struct :`X` 60.0 :`Y` 60.0 :`Z` 60.0 :`W` 60.0) :`Color` (struct :`SpecifiedColor` (struct) :`ColorUseRule` "UseColor_Specified") :`RoundingType` "HalfHeightRadius") :`UVRegion` (struct :`Min` (0.0 0.0) :`Max` (0.0 0.0)) :`DrawAs` "Box" :`Tiling` "NoTile" :`Mirroring` "NoMirror" :`ImageType` "NoImage") :`Hovered` (struct :`ImageSize` (32.0 32.0) :`Margin` (struct) :`TintColor` (struct :`SpecifiedColor` (struct :`R` 0.83077 :`G` 0.198069) :`ColorUseRule` "UseColor_Specified") :`OutlineSettings` (struct :`CornerRadii` (struct :`X` 60.0 :`Y` 60.0 :`Z` 60.0 :`W` 60.0) :`Color` (struct :`SpecifiedColor` (struct) :`ColorUseRule` "UseColor_Specified") :`RoundingType` "HalfHeightRadius") :`UVRegion` (struct :`Min` (0.0 0.0) :`Max` (0.0 0.0)) :`DrawAs` "RoundedBox" :`Tiling` "NoTile" :`Mirroring` "NoMirror" :`ImageType` "NoImage") :`Pressed` (struct :`ImageSize` (32.0 32.0) :`Margin` (struct) :`TintColor` (struct :`SpecifiedColor` (struct :`R` 0.62396 :`G` 0.014444 :`B` 0.08022) :`ColorUseRule` "UseColor_Specified") :`OutlineSettings` (struct :`CornerRadii` (struct :`X` 60.0 :`Y` 60.0 :`Z` 60.0 :`W` 60.0) :`Color` (struct :`SpecifiedColor` (struct) :`ColorUseRule` "UseColor_Specified") :`RoundingType` "HalfHeightRadius") :`UVRegion` (struct :`Min` (0.0 0.0) :`Max` (0.0 0.0)) :`DrawAs` "RoundedBox" :`Tiling` "NoTile" :`Mirroring` "NoMirror" :`ImageType` "NoImage") :`Disabled` (struct :`ImageSize` (0.0 0.0) :`Margin` (struct) :`TintColor` (struct :`SpecifiedColor` (struct :`R` 1.0 :`G` 1.0 :`B` 1.0 :`A` 1.0) :`ColorUseRule` "UseColor_Specified") :`OutlineSettings` (struct :`CornerRadii` (struct :`W` 1.0) :`Color` (struct :`SpecifiedColor` (struct) :`ColorUseRule` "UseColor_Specified") :`RoundingType` "HalfHeightRadius") :`UVRegion` (struct :`Min` (0.0 0.0) :`Max` (0.0 0.0)) :`DrawAs` "NoDrawType" :`Tiling` "NoTile" :`Mirroring` "NoMirror" :`ImageType` "NoImage") :`NormalForeground` (struct :`SpecifiedColor` (struct :`R` 1.0 :`B` 1.0 :`A` 1.0) :`ColorUseRule` "UseColor_Foreground") :`HoveredForeground` (struct :`SpecifiedColor` (struct :`R` 1.0 :`B` 1.0 :`A` 1.0) :`ColorUseRule` "UseColor_Foreground") :`PressedForeground` (struct :`SpecifiedColor` (struct :`R` 1.0 :`B` 1.0 :`A` 1.0) :`ColorUseRule` "UseColor_Foreground") :`DisabledForeground` (struct :`SpecifiedColor` (struct :`R` 1.0 :`B` 1.0 :`A` 1.0) :`ColorUseRule` "UseColor_Foreground") :`NormalPadding` (struct) :`PressedPadding` (struct) :`PressedSlateSound` (struct) :`HoveredSlateSound` (struct))) (MouseStyle_new :type "ButtonStyle Structure" :default (struct :`Normal` (struct :`ImageSize` (32.0 32.0) :`Margin` (struct) :`TintColor` (struct :`SpecifiedColor` (struct :`R` 1.0 :`G` 0.590619 :`B` 0.162029) :`ColorUseRule` "UseColor_Specified") :`OutlineSettings` (struct :`CornerRadii` (struct :`X` 60.0 :`Y` 60.0 :`Z` 60.0 :`W` 60.0) :`Color` (struct :`SpecifiedColor` (struct) :`ColorUseRule` "UseColor_Specified") :`RoundingType` "HalfHeightRadius") :`UVRegion` (struct :`Min` (0.0 0.0) :`Max` (0.0 0.0)) :`DrawAs` "Box" :`Tiling` "NoTile" :`Mirroring` "NoMirror" :`ImageType` "NoImage") :`Hovered` (struct :`ImageSize` (32.0 32.0) :`Margin` (struct) :`TintColor` (struct :`SpecifiedColor` (struct :`R` 0.83077 :`G` 0.198069 :`A` 0.025) :`ColorUseRule` "UseColor_Specified") :`OutlineSettings` (struct :`CornerRadii` (struct :`X` 60.0 :`Y` 60.0 :`Z` 60.0 :`W` 60.0) :`Color` (struct :`SpecifiedColor` (struct) :`ColorUseRule` "UseColor_Specified") :`RoundingType` "HalfHeightRadius") :`UVRegion` (struct :`Min` (0.0 0.0) :`Max` (0.0 0.0)) :`DrawAs` "Box" :`Tiling` "NoTile" :`Mirroring` "NoMirror" :`ImageType` "NoImage") :`Pressed` (struct :`ImageSize` (32.0 32.0) :`Margin` (struct) :`TintColor` (struct :`SpecifiedColor` (struct :`R` 0.62396 :`G` 0.014444 :`B` 0.08022) :`ColorUseRule` "UseColor_Specified") :`OutlineSettings` (struct :`CornerRadii` (struct :`X` 60.0 :`Y` 60.0 :`Z` 60.0 :`W` 60.0) :`Color` (struct :`SpecifiedColor` (struct) :`ColorUseRule` "UseColor_Specified") :`RoundingType` "HalfHeightRadius") :`UVRegion` (struct :`Min` (0.0 0.0) :`Max` (0.0 0.0)) :`DrawAs` "Box" :`Tiling` "NoTile" :`Mirroring` "NoMirror" :`ImageType` "NoImage") :`Disabled` (struct :`ImageSize` (0.0 0.0) :`Margin` (struct) :`TintColor` (struct :`SpecifiedColor` (struct :`R` 1.0 :`G` 1.0 :`B` 1.0 :`A` 1.0) :`ColorUseRule` "UseColor_Specified") :`OutlineSettings` (struct :`CornerRadii` (struct :`W` 1.0) :`Color` (struct :`SpecifiedColor` (struct) :`ColorUseRule` "UseColor_Specified") :`RoundingType` "HalfHeightRadius") :`UVRegion` (struct :`Min` (0.0 0.0) :`Max` (0.0 0.0)) :`DrawAs` "NoDrawType" :`Tiling` "NoTile" :`Mirroring` "NoMirror" :`ImageType` "NoImage") :`NormalForeground` (struct :`SpecifiedColor` (struct :`R` 1.0 :`B` 1.0 :`A` 1.0) :`ColorUseRule` "UseColor_Foreground") :`HoveredForeground` (struct :`SpecifiedColor` (struct :`R` 1.0 :`B` 1.0 :`A` 1.0) :`ColorUseRule` "UseColor_Foreground") :`PressedForeground` (struct :`SpecifiedColor` (struct :`R` 1.0 :`B` 1.0 :`A` 1.0) :`ColorUseRule` "UseColor_Foreground") :`DisabledForeground` (struct :`SpecifiedColor` (struct :`R` 1.0 :`B` 1.0 :`A` 1.0) :`ColorUseRule` "UseColor_Foreground") :`NormalPadding` (struct) :`PressedPadding` (struct) :`PressedSlateSound` (struct) :`HoveredSlateSound` (struct))) (KeySelected_new :type "ButtonStyle Structure" :default (struct :`Normal` (struct :`ImageSize` (32.0 32.0) :`Margin` (struct) :`TintColor` (struct :`SpecifiedColor` (struct :`R` 0.83077 :`G` 0.198069) :`ColorUseRule` "UseColor_Specified") :`OutlineSettings` (struct :`CornerRadii` (struct :`X` 60.0 :`Y` 60.0 :`Z` 60.0 :`W` 60.0) :`Color` (struct :`SpecifiedColor` (struct) :`ColorUseRule` "UseColor_Specified") :`RoundingType` "HalfHeightRadius") :`UVRegion` (struct :`Min` (0.0 0.0) :`Max` (0.0 0.0)) :`DrawAs` "Box" :`Tiling` "NoTile" :`Mirroring` "NoMirror" :`ImageType` "NoImage") :`Hovered` (struct :`ImageSize` (32.0 32.0) :`Margin` (struct) :`TintColor` (struct :`SpecifiedColor` (struct :`R` 0.83077 :`G` 0.198069 :`A` 0.004) :`ColorUseRule` "UseColor_Specified") :`OutlineSettings` (struct :`CornerRadii` (struct :`X` 60.0 :`Y` 60.0 :`Z` 60.0 :`W` 60.0) :`Color` (struct :`SpecifiedColor` (struct) :`ColorUseRule` "UseColor_Specified") :`RoundingType` "HalfHeightRadius") :`UVRegion` (struct :`Min` (0.0 0.0) :`Max` (0.0 0.0)) :`DrawAs` "Box" :`Tiling` "NoTile" :`Mirroring` "NoMirror" :`ImageType` "NoImage") :`Pressed` (struct :`ImageSize` (32.0 32.0) :`Margin` (struct) :`TintColor` (struct :`SpecifiedColor` (struct :`R` 0.62396 :`G` 0.014444 :`B` 0.08022) :`ColorUseRule` "UseColor_Specified") :`OutlineSettings` (struct :`CornerRadii` (struct :`X` 60.0 :`Y` 60.0 :`Z` 60.0 :`W` 60.0) :`Color` (struct :`SpecifiedColor` (struct) :`ColorUseRule` "UseColor_Specified") :`RoundingType` "HalfHeightRadius") :`UVRegion` (struct :`Min` (0.0 0.0) :`Max` (0.0 0.0)) :`DrawAs` "Box" :`Tiling` "NoTile" :`Mirroring` "NoMirror" :`ImageType` "NoImage") :`Disabled` (struct :`ImageSize` (0.0 0.0) :`Margin` (struct) :`TintColor` (struct :`SpecifiedColor` (struct :`R` 1.0 :`G` 1.0 :`B` 1.0 :`A` 1.0) :`ColorUseRule` "UseColor_Specified") :`OutlineSettings` (struct :`CornerRadii` (struct :`W` 1.0) :`Color` (struct :`SpecifiedColor` (struct) :`ColorUseRule` "UseColor_Specified") :`RoundingType` "HalfHeightRadius") :`UVRegion` (struct :`Min` (0.0 0.0) :`Max` (0.0 0.0)) :`DrawAs` "NoDrawType" :`Tiling` "NoTile" :`Mirroring` "NoMirror" :`ImageType` "NoImage") :`NormalForeground` (struct :`SpecifiedColor` (struct :`R` 1.0 :`B` 1.0 :`A` 1.0) :`ColorUseRule` "UseColor_Foreground") :`HoveredForeground` (struct :`SpecifiedColor` (struct :`R` 1.0 :`B` 1.0 :`A` 1.0) :`ColorUseRule` "UseColor_Foreground") :`PressedForeground` (struct :`SpecifiedColor` (struct :`R` 1.0 :`B` 1.0 :`A` 1.0) :`ColorUseRule` "UseColor_Foreground") :`DisabledForeground` (struct :`SpecifiedColor` (struct :`R` 1.0 :`B` 1.0 :`A` 1.0) :`ColorUseRule` "UseColor_Foreground") :`NormalPadding` (struct) :`PressedPadding` (struct) :`PressedSlateSound` (struct) :`HoveredSlateSound` (struct))))
  (if (`Widget.IsHovered` NewParam)
    (`Widget.SetKeyboardFocus` NewParam)
    (`Button.SetStyle` NewParam (`local.MouseStyle_new`))
    (else
      (`Button.SetStyle` NewParam (select `bool` (`Widget.HasKeyboardFocus` NewParam) :`false` (`local.KeyNotStyle`) :`true` (`local.KeySelected_new`))))))

(fn `Play Music`
  (params (`If UI` :type Boolean))
  (returns (UI_BGM :type "AudioComponent Object Reference") (Play_BGM :type "AudioComponent Object Reference"))
  (locals (BGM :type "Array of SoundWave Object Reference") (BGM_UI :type "AudioComponent Object Reference") (BGM_Play :type "AudioComponent Object Reference"))
  (bind _bgm (`local.BGM`))
  (if `If UI`
    (bind _returnvalue (`GameplayStatics.CreateSound2D` null (`|GetArrayItem` _bgm) 1.0 1.0 0.0 null))
    (bind _output_get (set `local.BGM_UI` _returnvalue))
    (`AudioComponent.FadeIn` _output_get 1.68 1.0 0.0 "Linear")
    (else
      (bind _returnvalue_2 (`GameplayStatics.CreateSound2D` null (`|GetArrayItem` _bgm 1) 1.0 1.0 0.0 null))
      (bind _output_get_2 (set `local.BGM_Play` _returnvalue_2))
      (`AudioComponent.FadeIn` _output_get_2 1.68 1.0 0.0 "Linear")))
  (return _output_get _output_get_2))