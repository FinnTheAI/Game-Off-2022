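; BP_GuineaPigBlock is a bounce block that launches the 2D side-scroller character upward.
; A capsule overlap by a living, non-rising character briefly sets its IfQitiao (take-off) flag, activates the 弹跳04 (bounce) component, then after a short delay launches it and swaps sprites.
; Ending overlap with PaperSprite_01 restores the idle sprite after a delay.
; Overlap by a dead character disables the block's collision.
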(event `self.ReceiveBeginPlay`
  (`SceneComponent.SetVisibility` (`self.PaperSprite_01`) true false)
  (`SceneComponent.SetVisibility` (`self.PaperSprite_02`) false false)
  (`ActorComponent.SetActive` (`self.弹跳04`) false true))

(event `self.ReceiveTick`
  (params (DeltaSeconds :type "Float (single-precision)")))

(event `self.Capsule.OnComponentBeginOverlap`
  (params (OverlappedComponent :type "PrimitiveComponent Object Reference") (OtherActor :type "Actor Object Reference") (OtherComp :type "PrimitiveComponent Object Reference") (OtherBodyIndex :type Integer) (bFromSweep :type Boolean) (SweepResult :type "HitResult Structure (by ref)"))
  (bind _as2dside_scroller_character (cast `/Game/2DSideScrollerBP/Blueprints/2DSideScrollerCharacter` OtherActor))
  (if (`/Game/2DSideScrollerBP/Blueprints/2DSideScrollerCharacter.If Dead` _as2dside_scroller_character)
    (`self.SetActorEnableCollision` false)
    (else
      (bind (_returnvalue_x _returnvalue_y _returnvalue_z) (`KismetMathLibrary.BreakVector` (`self.GetVelocity` _as2dside_scroller_character)))
      (if (not (> _returnvalue_z 0.0))
        ;[1 1 1] Comment
        (set `/Game/2DSideScrollerBP/Blueprints/2DSideScrollerCharacter.If Qitiao` true _as2dside_scroller_character)
        (`|ExecutionSequence`
          (:`then_0`
            (`KismetSystemLibrary.Delay` 0.4)
            (set `/Game/2DSideScrollerBP/Blueprints/2DSideScrollerCharacter.If Qitiao` false _as2dside_scroller_character))
          (:`then_1`
            (`KismetSystemLibrary.Delay` 0.13)
            (`Character.LaunchCharacter` _as2dside_scroller_character (0.0 0.0 3500.0) false true)
            (`SceneComponent.SetVisibility` (`self.PaperSprite_01`) false false)
            (`SceneComponent.SetVisibility` (`self.PaperSprite_02`) true false))
          (:`then_2`
            (`ActorComponent.SetActive` (`self.弹跳04`) true true)))))))

(event `self.PaperSprite_01.OnComponentEndOverlap`
  (params (OverlappedComponent :type "PrimitiveComponent Object Reference") (OtherActor :type "Actor Object Reference") (OtherComp :type "PrimitiveComponent Object Reference") (OtherBodyIndex :type Integer))
  (`KismetSystemLibrary.Delay` 0.5)
  (`SceneComponent.SetVisibility` (`self.PaperSprite_01`) true false)
  (`SceneComponent.SetVisibility` (`self.PaperSprite_02`) false false))

(fn `UserConstructionScript`)