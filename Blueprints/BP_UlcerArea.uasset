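; BP_UlcerArea is a side-scroller hazard: an ulcer that bursts when the player character steps on it and sprays liquid that covers the view.
; Capsule overlap briefly swaps the ulcer visuals, then activates the burst effect and shows a splatter flipbook, which switches to a fade-out animation before hiding.
; Tick keeps the splatter at a height offset from the player, and a flag blocks retriggering until the sequence resets.
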(event `self.ReceiveBeginPlay`
  (`SceneComponent.SetVisibility` (`self.Ulcer_Boom_00`) false false)
  (`SceneComponent.SetVisibility` (`self.Ulcer_01`) true false)
  (`SceneComponent.SetVisibility` (`self.Ulcer_02`) false false)
  (`ActorComponent.SetActive` (`self.溃疡爆开`) false true))

(event `self.ReceiveTick`
  (params (DeltaSeconds :type "Float (single-precision)"))
  (bind _returnvalue (`GameplayStatics.GetPlayerPawn` 0))
  (bind (_returnvalue_x _returnvalue_y _returnvalue_z) (`KismetMathLibrary.BreakVector` (`self.K2_GetActorLocation` _returnvalue)))
  ;[1 1 1] 溃疡液体位置
  (`/Engine/EditorBlueprintResources/StandardMacros.IsValid` _returnvalue
    (:`Is Valid`
      (`SceneComponent.K2_SetWorldLocation` (`self.Ulcer_Boom_00`) (`KismetMathLibrary.MakeVector` 0.0 1000.0 (+ _returnvalue_z 800.0)) false false))))

(event `self.Capsule.OnComponentBeginOverlap`
  (params (OverlappedComponent :type "PrimitiveComponent Object Reference") (OtherActor :type "Actor Object Reference") (OtherComp :type "PrimitiveComponent Object Reference") (OtherBodyIndex :type Integer) (bFromSweep :type Boolean) (SweepResult :type "HitResult Structure (by ref)"))
  (bind _ulcer_boom_00 (`self.Ulcer_Boom_00`))
  (cast `/Game/2DSideScrollerBP/Blueprints/2DSideScrollerCharacter` OtherActor)
  (if (not (`self.If Ulcer`))
    (set `self.If Ulcer` true)
    ;[1 1 1] 踩爆
    (`SceneComponent.SetVisibility` (`self.Ulcer_01`) false false)
    (`SceneComponent.SetVisibility` (`self.Ulcer_02`) true false)
    (`KismetSystemLibrary.Delay` 0.3)
    ;[1 1 1] 飙汁
    (`SceneComponent.SetVisibility` (`self.Ulcer_01`) true false)
    (`SceneComponent.SetVisibility` (`self.Ulcer_02`) false false)
    (`ActorComponent.SetActive` (`self.溃疡爆开`) true true)
    ;[1 1 1] 1.3s遮盖，1.2s渐消
    (`SceneComponent.SetVisibility` _ulcer_boom_00 true false)
    (`KismetSystemLibrary.Delay` 1.3)
    (`PaperFlipbookComponent.SetFlipbook` _ulcer_boom_00 "/Game/2DSideScroller/Sprites/Frames_Ulcer/Ulcer_Boom.Ulcer_Boom")
    (`KismetSystemLibrary.Delay` 1.2)
    (`SceneComponent.SetVisibility` _ulcer_boom_00 false false)
    (`PaperFlipbookComponent.SetFlipbook` _ulcer_boom_00 "/Game/2DSideScroller/Sprites/Frames_Ulcer/Ulcer_Boom_00.Ulcer_Boom_00")
    (set `self.If Ulcer` false)))

(fn `UserConstructionScript`)