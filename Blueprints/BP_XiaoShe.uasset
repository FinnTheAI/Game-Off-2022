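; BP_XiaoShe is the "small tongue" goal actor that marks the side-scroller character as having won on contact.
; A capsule overlap with a living 2DSideScrollerCharacter sets IfWin, increments SmallTongue in the GameInstance's user database and saves it to the slot.
; The increment and save repeat on every living overlap, even after a win.
; Overlap with a dead character disables the actor's collision instead.
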(event `self.ReceiveBeginPlay`
  (bind _asbp_game_instance (cast `/Game/2DSideScrollerBP/Blueprints/BP_Core/BP_GameInstance` (`GameplayStatics.GetGameInstance`))
    (:`then`
      (set `self.As BP Game Instance` _asbp_game_instance))
    (:`CastFailed`
      (`KismetSystemLibrary.PrintString` "Error: Can't cast to GameInstance."))))

(event `self.ReceiveTick`
  (params (DeltaSeconds :type "Float (single-precision)")))

(event `self.Capsule.OnComponentBeginOverlap`
  (params (OverlappedComponent :type "PrimitiveComponent Object Reference") (OtherActor :type "Actor Object Reference") (OtherComp :type "PrimitiveComponent Object Reference") (OtherBodyIndex :type Integer) (bFromSweep :type Boolean) (SweepResult :type "HitResult Structure (by ref)"))
  (bind _as_bp_game_instance (`self.As BP Game Instance`))
  (bind _users_data_base (`/Game/2DSideScrollerBP/Blueprints/BP_Core/BP_GameInstance.Users Data Base` _as_bp_game_instance))
  (bind _as2dside_scroller_character (cast `/Game/2DSideScrollerBP/Blueprints/2DSideScrollerCharacter` OtherActor))
  (if (`/Game/2DSideScrollerBP/Blueprints/2DSideScrollerCharacter.If Dead` _as2dside_scroller_character)
    (`self.SetActorEnableCollision` false)
    (else
      (if (not (`/Game/2DSideScrollerBP/Blueprints/2DSideScrollerCharacter.If Win` _as2dside_scroller_character))
        (set `/Game/2DSideScrollerBP/Blueprints/2DSideScrollerCharacter.If Win` true _as2dside_scroller_character))
      (`/Engine/EditorBlueprintResources/StandardMacros.IncrementInt` (`/Game/2DSideScrollerBP/Blueprints/BP_Core/SG_UsersData.Small Tongue` _users_data_base)
        (:`  `
          (`GameplayStatics.SaveGameToSlot` _users_data_base (`/Game/2DSideScrollerBP/Blueprints/BP_Core/BP_GameInstance.Slot Name` _as_bp_game_instance)))))))

(fn `UserConstructionScript`)