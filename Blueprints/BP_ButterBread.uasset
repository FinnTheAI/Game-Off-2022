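; BP_ButterBread is a 2D side-scroller pickup that launches the player upward on overlap with its box.
; The overlap sets IfButterBread on the character and itself, or disables its collision if the character is dead.
; While flagged, Tick hides the sprite, forces upward character velocity and activates the 翻飞 component.
; After a 2.5-second delay it destroys itself and clears both flags.
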(event `self.ReceiveBeginPlay`
  (`ActorComponent.SetActive` (`self.翻飞`) false true))

(event `self.ReceiveTick`
  (params (DeltaSeconds :type "Float (single-precision)"))
  ;[1 1 1] 判断是否在黄油面包状态
  (`/Engine/EditorBlueprintResources/StandardMacros.IsValid` (stale `self.Box.OnComponentBeginOverlap` _as2dside_scroller_character)
    (:`Is Valid`
      (if (`self.If Butter Bread`)
        (`SceneComponent.SetVisibility` (`self.PaperSprite`) false false)
        (bind (_returnvalue_x _returnvalue_y) (`KismetMathLibrary.BreakVector` (`self.GetVelocity` (stale `self.Box.OnComponentBeginOverlap` _as2dside_scroller_character))))
        (set `MovementComponent.Velocity` (`KismetMathLibrary.MakeVector` _returnvalue_x _returnvalue_y 2300.0) (`Pawn.GetMovementComponent` (stale `self.Box.OnComponentBeginOverlap` _as2dside_scroller_character)))
        (`ActorComponent.SetActive` (`self.翻飞`) true false)
        (`KismetSystemLibrary.Delay` 2.5)
        (`self.K2_DestroyActor`)
        (bind _output_get (set `self.If Butter Bread` false))
        (set `/Game/2DSideScrollerBP/Blueprints/2DSideScrollerCharacter.If ButterBread` _output_get (stale `self.Box.OnComponentBeginOverlap` _as2dside_scroller_character))))))

(event `self.Box.OnComponentBeginOverlap`
  (params (OverlappedComponent :type "PrimitiveComponent Object Reference") (OtherActor :type "Actor Object Reference") (OtherComp :type "PrimitiveComponent Object Reference") (OtherBodyIndex :type Integer) (bFromSweep :type Boolean) (SweepResult :type "HitResult Structure (by ref)"))
  ;[1 1 1] 开始碰撞进入黄油面包状态，并Get Movement Component
  (bind _as2dside_scroller_character (cast `/Game/2DSideScrollerBP/Blueprints/2DSideScrollerCharacter` OtherActor))
  (if (`/Game/2DSideScrollerBP/Blueprints/2DSideScrollerCharacter.If Dead` _as2dside_scroller_character)
    (`self.SetActorEnableCollision` false)
    (else
      (bind _output_get (set `/Game/2DSideScrollerBP/Blueprints/2DSideScrollerCharacter.If ButterBread` true _as2dside_scroller_character))
      (set `self.If Butter Bread` _output_get))))

(fn `UserConstructionScript`)