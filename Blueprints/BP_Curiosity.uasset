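; BP_Curiosity is an actor that displays a Curiosity flipbook sprite alternating between animated and static looks.
; At BeginPlay, if its Scene component sits at world X of zero or above, the sprite gets a new rotated, scaled relative transform.
; Tick drives a latent Delay into a FlipFlop, so the flipbook swaps between PF_Curiosity and PF_Curiosity_Static on a timed cycle.
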(event `self.ReceiveBeginPlay`
  (bind _returnvalue_x (`KismetMathLibrary.BreakVector` (`SceneComponent.K2_GetComponentLocation` (`self.Scene`))))
  (if (>= _returnvalue_x 0.0)
    (`SceneComponent.K2_SetRelativeTransform` (`self.Curiosity`) (`KismetMathLibrary.MakeTransform` (-85.0 -200.0 30.0) (struct :`Yaw` 180.0) (0.35 0.35 0.35)) false false)))

(event `self.ReceiveTick`
  (params (DeltaSeconds :type "Float (single-precision)"))
  (bind _curiosity (`self.Curiosity`))
  (`KismetSystemLibrary.Delay` 2.0)
  (`/Engine/EditorBlueprintResources/StandardMacros.FlipFlop`
    (:`A`
      (`PaperFlipbookComponent.SetFlipbook` _curiosity "/Game/2DSideScroller/Sprites/Frames_Curiosity/PF_Curiosity.PF_Curiosity"))
    (:`B`
      (`PaperFlipbookComponent.SetFlipbook` _curiosity "/Game/2DSideScroller/Sprites/Frames_Curiosity/PF_Curiosity_Static.PF_Curiosity_Static")))
  (`KismetSystemLibrary.Delay` 1.0))

(fn `UserConstructionScript`)