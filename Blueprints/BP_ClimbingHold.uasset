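; A bounce foothold for the 2D side-scroller that launches the player upward on landing, with a random 0 or 180 degree yaw at start.
; A capsule overlap by a living character, not rising or falling too fast, sets its takeoff flag, plays bounce audio and launches it after a short delay.
; Tick swaps the two pedal visuals from the trodden flag, cleared by a retriggerable delay.
; Overlap by a dead character disables the hold's collision.
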(event `self.ReceiveBeginPlay`
  (`SceneComponent.SetVisibility` (`self.Pedal_01`) true false)
  (`SceneComponent.SetVisibility` (`self.Pedal_02`) false false)
  ;[1 1 1] Comment
  (`SceneComponent.K2_SetRelativeRotation` (`self.DefaultSceneRoot`) (`KismetMathLibrary.MakeRotator` 0.0 0.0 (`KismetMathLibrary.Conv_IntToDouble` (* (`KismetMathLibrary.RandomIntegerInRange` 0 1) 180))) false false)
  (`ActorComponent.SetActive` (`self.弹跳02`) false true))

(event `self.ReceiveTick`
  (params (DeltaSeconds :type "Float (single-precision)"))
  (if (`self.If Treaded`)
    (`SceneComponent.SetVisibility` (`self.Pedal_01`) false false)
    (`SceneComponent.SetVisibility` (`self.Pedal_02`) true false)
    (else
      (`SceneComponent.SetVisibility` (`self.Pedal_01`) true false)
      (`SceneComponent.SetVisibility` (`self.Pedal_02`) false false))))

(event `self.Capsule.OnComponentBeginOverlap`
  (params (OverlappedComponent :type "PrimitiveComponent Object Reference") (OtherActor :type "Actor Object Reference") (OtherComp :type "PrimitiveComponent Object Reference") (OtherBodyIndex :type Integer) (bFromSweep :type Boolean) (SweepResult :type "HitResult Structure (by ref)"))
  (bind _as2dside_scroller_character (cast `/Game/2DSideScrollerBP/Blueprints/2DSideScrollerCharacter` OtherActor))
  (if (`/Game/2DSideScrollerBP/Blueprints/2DSideScrollerCharacter.If Dead` _as2dside_scroller_character)
    (`self.SetActorEnableCollision` false)
    (else
      (bind (_returnvalue_x _returnvalue_y _returnvalue_z) (`KismetMathLibrary.BreakVector` (`self.GetVelocity` _as2dside_scroller_character)))
      ;[1 1 1] 下落判定+超速检验
      (if (> _returnvalue_z 0.0)
        _
        (elif (> _returnvalue_z -4000.0)
          ;[1 1 1] 落地起跳动作维持0.4s
          (bind _output_get (set `/Game/2DSideScrollerBP/Blueprints/2DSideScrollerCharacter.If Qitiao` true _as2dside_scroller_character))
          (set `self.If Treaded` _output_get)
          (`|ExecutionSequence`
            (:`then_0`
              (`KismetSystemLibrary.RetriggerableDelay` 0.4)
              (bind _output_get_2 (set `/Game/2DSideScrollerBP/Blueprints/2DSideScrollerCharacter.If Qitiao` false _as2dside_scroller_character))
              (set `self.If Treaded` _output_get_2))
            (:`then_1`
              (`KismetSystemLibrary.Delay` 0.1)
              (`Character.LaunchCharacter` _as2dside_scroller_character (0.0 0.0 2200.0) false true))
            (:`then_2`
              ;[1 1 1] Audio
              (`ActorComponent.SetActive` (`self.弹跳02`) true true))))))))

(fn `UserConstructionScript`)