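; BP_Enemy is a side-scroller enemy that moves by a fixed transform each throttled tick and destroys itself at spawn while the game is in UI.
; Overlaps on EnemyMove rotate that component's yaw to reverse it.
; When IsDead is set, it shows EnemyHitted, disables collision, activates Hitted if the player lives, then destroys itself after a delay.
; Capsule overlap caches the player; its falling-speed check triggers nothing.
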(event `self.ReceiveBeginPlay`
  (`|ExecutionSequence`
    (:`then_0`
      ;[1 1 1] Comment
      (bind _asbp_game_instance (cast `/Game/2DSideScrollerBP/Blueprints/BP_Core/BP_GameInstance` (`GameplayStatics.GetGameInstance`)))
      (set `self.As BP Game Instance` _asbp_game_instance))
    (:`then_1`
      (if (`/Game/2DSideScrollerBP/Blueprints/BP_Core/BP_GameInstance.If in UI` (`self.As BP Game Instance`))
        (`ActorComponent.SetActive` (`self.EnemyMove`) false false)
        (`ActorComponent.SetActive` (`self.EnemyHitted`) false false)
        (`ActorComponent.SetActive` (`self.Hitted`) false false)
        (`self.K2_DestroyActor`)
        (else
          (`SceneComponent.SetVisibility` (`self.EnemyMove`) true false)
          (`SceneComponent.SetVisibility` (`self.EnemyHitted`) false false)
          (`ActorComponent.SetActive` (`self.Hitted`) false true))))
    (:`then_2`
      (`self.SetActorTickInterval` 0.02))))

(event `self.ReceiveTick`
  (params (DeltaSeconds :type "Float (single-precision)"))
  (if (`self.Is Dead`)
    ;[1 1 1] 敌人死亡判定
    (`SceneComponent.SetVisibility` (`self.EnemyMove`) false false)
    (`SceneComponent.SetVisibility` (`self.EnemyHitted`) true false)
    (`self.SetActorEnableCollision` false)
    (if (not (`/Game/2DSideScrollerBP/Blueprints/2DSideScrollerCharacter.If Dead` (stale `self.Capsule.OnComponentBeginOverlap` _as2dside_scroller_character)))
      (`ActorComponent.SetActive` (`self.Hitted`) true false))
    (`KismetSystemLibrary.Delay` 0.4)
    (`self.K2_DestroyActor`)
    (else
      ;[1 1 1] 敌人初始移动
      (`SceneComponent.K2_AddLocalTransform` (`self.Scene`) (`self.Scene Transform`) false false))))

(event `self.EnemyMove.OnComponentBeginOverlap`
  (params (OverlappedComponent :type "PrimitiveComponent Object Reference") (OtherActor :type "Actor Object Reference") (OtherComp :type "PrimitiveComponent Object Reference") (OtherBodyIndex :type Integer) (bFromSweep :type Boolean) (SweepResult :type "HitResult Structure (by ref)"))
  (bind _returnvalue (+ (`self.Temp Rotation Z (Yaw)`) 180.0))
  ;[1 1 1] Sprite反向？
  (set `self.If Reverse` true)
  (if (`self.If Reverse`)
    (set `self.Temp Rotation Z (Yaw)` _returnvalue)
    (`SceneComponent.K2_SetRelativeRotation` (`self.EnemyMove`) (`KismetMathLibrary.MakeRotator` 0.0 0.0 _returnvalue) false false)
    (set `self.If Reverse` false)))

(event `self.Capsule.OnComponentBeginOverlap`
  (params (OverlappedComponent :type "PrimitiveComponent Object Reference") (OtherActor :type "Actor Object Reference") (OtherComp :type "PrimitiveComponent Object Reference") (OtherBodyIndex :type Integer) (bFromSweep :type Boolean) (SweepResult :type "HitResult Structure (by ref)"))
  (bind (_returnvalue_x _returnvalue_y _returnvalue_z) (`KismetMathLibrary.BreakVector` (`self.GetVelocity`)))
  (bind _as2dside_scroller_character (cast `/Game/2DSideScrollerBP/Blueprints/2DSideScrollerCharacter` OtherActor))
  (if (`/Game/2DSideScrollerBP/Blueprints/2DSideScrollerCharacter.If Dead` _as2dside_scroller_character)
    (`self.SetActorEnableCollision` false)
    (else
      ;[1 1 1] 下落判定+超速检验
      (if (>= _returnvalue_z 0.0)
        _
        (elif (> _returnvalue_z -4000.0)
          _)))))

(fn `UserConstructionScript`)