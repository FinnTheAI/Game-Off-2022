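; Launcher enemy for a 2D side-scroller that starts at a random 0 or 180 degree rotation and doubles as a bounce pad.
; Tick uses Delays to alternate two launcher visuals and spawn a child actor at the Arrow's location.
; Box overlap launches a living character upward with audio and flags a trodden visual, gated by the launcher's own Z velocity.
; Box_Bullet marks overlapping BP_Enemy_Bullet actors dead.
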(event `self.ReceiveBeginPlay`
  (`SceneComponent.SetVisibility` (`self.Launcher_01`) true false)
  (`SceneComponent.SetVisibility` (`self.Launcher_02`) false false)
  (`ActorComponent.SetActive` (`self.弹跳01`) false true)
  (if (`KismetMathLibrary.RandomBool`)
    (`self.K2_SetActorRelativeRotation` (struct))
    (else
      (`self.K2_SetActorRelativeRotation` (struct :`Yaw` 180.0)))))

(event `self.ReceiveTick`
  (params (DeltaSeconds :type "Float (single-precision)"))
  (bind _launcher_01 (`self.Launcher_01`))
  (bind _launcher_02 (`self.Launcher_02`))
  (if (`self.Is Treaded`)
    ;[1 1 1] Comment
    (`SceneComponent.SetVisibility` _launcher_01 false false)
    (`SceneComponent.SetVisibility` _launcher_02 false false)
    (`SceneComponent.SetVisibility` (`self.Launcher_03`) true false)
    (`KismetSystemLibrary.Delay` 0.4)
    (`SceneComponent.SetVisibility` _launcher_01 true false)
    (`SceneComponent.SetVisibility` _launcher_02 false false)
    (`SceneComponent.SetVisibility` (`self.Launcher_03`) false false)
    (set `self.Is Treaded` false)
    (else
      (`KismetSystemLibrary.Delay` 0.6)
      ;[1 1 1] Comment
      (`SceneComponent.SetVisibility` _launcher_01 true false)
      (`SceneComponent.SetVisibility` _launcher_02 false false)
      (`KismetSystemLibrary.Delay` 0.7)
      (`SceneComponent.SetVisibility` _launcher_01 false false)
      (`SceneComponent.SetVisibility` _launcher_02 true false)
      (`AddComponent|NODE_AddChildActorComponent-0` :`RelativeTransform` (`KismetMathLibrary.MakeTransform` (`SceneComponent.RelativeLocation` (`self.Arrow`))))
      (`KismetSystemLibrary.Delay` 0.6))))

(event `self.Box.OnComponentBeginOverlap`
  (params (OverlappedComponent :type "PrimitiveComponent Object Reference") (OtherActor :type "Actor Object Reference") (OtherComp :type "PrimitiveComponent Object Reference") (OtherBodyIndex :type Integer) (bFromSweep :type Boolean) (SweepResult :type "HitResult Structure (by ref)"))
  (bind (_returnvalue_x _returnvalue_y _returnvalue_z) (`KismetMathLibrary.BreakVector` (`self.GetVelocity`)))
  ;[1 1 1] 触碰死亡
  (bind _as2dside_scroller_character (cast `/Game/2DSideScrollerBP/Blueprints/2DSideScrollerCharacter` OtherActor))
  (if (`/Game/2DSideScrollerBP/Blueprints/2DSideScrollerCharacter.If Dead` _as2dside_scroller_character)
    (`self.SetActorEnableCollision` false)
    (elif (> _returnvalue_z 0.0)
      _
      (elif (> _returnvalue_z -4000.0)
        (set `self.Is Treaded` true)
        ;[1 1 1] Comment
        (set `/Game/2DSideScrollerBP/Blueprints/2DSideScrollerCharacter.If Qitiao` true _as2dside_scroller_character)
        (`|ExecutionSequence`
          (:`then_0`
            (`KismetSystemLibrary.Delay` 0.4)
            (set `/Game/2DSideScrollerBP/Blueprints/2DSideScrollerCharacter.If Qitiao` false _as2dside_scroller_character))
          (:`then_1`
            (`KismetSystemLibrary.Delay` 0.1)
            (`Character.LaunchCharacter` _as2dside_scroller_character (0.0 0.0 2000.0) false true))
          (:`then_2`
            ;[1 1 1] Audio
            (`ActorComponent.SetActive` (`self.弹跳01`) true true)))))))

(event `self.Box_Bullet.OnComponentBeginOverlap`
  (params (OverlappedComponent :type "PrimitiveComponent Object Reference") (OtherActor :type "Actor Object Reference") (OtherComp :type "PrimitiveComponent Object Reference") (OtherBodyIndex :type Integer) (bFromSweep :type Boolean) (SweepResult :type "HitResult Structure (by ref)"))
  (bind _asbp_enemy_bullet (cast `/Game/2DSideScrollerBP/Blueprints/BP_Enemy_Bullet` OtherActor))
  (set `/Game/2DSideScrollerBP/Blueprints/BP_Enemy_Bullet.Is Dead` true _asbp_enemy_bullet))

(fn `UserConstructionScript`)