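; Final map segment of level 03 in the 2D side-scroller, with side wrapping, fall death and a win child actor.
; The construction script randomizes the X position of two child actors.
; BeginPlay spawns a BP_Curiosity above the segment, in a random left or right X band.
; Side triggers teleport the character to the opposite arrow's X; the death trigger sets IfDead after a short delay if the fall is fast enough.
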(event `self.ReceiveBeginPlay`
  (bind (_returnvalue_x _returnvalue_y _returnvalue_z) (`KismetMathLibrary.BreakVector` (`self.K2_GetActorLocation`)))
  ;[1 1 1] 随机生成Ulcer，？，None
  (`|SpawnActorFromClass` "/Game/2DSideScrollerBP/Blueprints/BP_Curiosity.BP_Curiosity_C" (`KismetMathLibrary.MakeTransform` (`KismetMathLibrary.MakeVector` (`KismetArrayLibrary.Array_Random` (`|MakeArray` (`KismetMathLibrary.RandomFloatInRange` -950.0 -550.0) (`KismetMathLibrary.RandomFloatInRange` 950.0 550.0))) 0.0 (+ _returnvalue_z 850.0))) "Undefined" "OverrideRootScale" null null))

(event `self.Left_TeleportCol.OnComponentBeginOverlap`
  (params (OverlappedComponent :type "PrimitiveComponent Object Reference") (OtherActor :type "Actor Object Reference") (OtherComp :type "PrimitiveComponent Object Reference") (OtherBodyIndex :type Integer) (bFromSweep :type Boolean) (SweepResult :type "HitResult Structure (by ref)"))
  (bind _returnvalue_x (`KismetMathLibrary.BreakVector` (`SceneComponent.K2_GetComponentLocation` (`self.Arrow_R`))))
  ;[1 1 1] 左右端传送
  (bind _as2dside_scroller_character (cast `/Game/2DSideScrollerBP/Blueprints/2DSideScrollerCharacter` OtherActor))
  (bind (_returnvalue_x_2 _returnvalue_y _returnvalue_z) (`KismetMathLibrary.BreakVector` (`self.K2_GetActorLocation` _as2dside_scroller_character)))
  (`self.K2_SetActorLocation` _as2dside_scroller_character (`KismetMathLibrary.MakeVector` _returnvalue_x _returnvalue_y _returnvalue_z) false true))

(event `self.Right_TeleportCol.OnComponentBeginOverlap`
  (params (OverlappedComponent :type "PrimitiveComponent Object Reference") (OtherActor :type "Actor Object Reference") (OtherComp :type "PrimitiveComponent Object Reference") (OtherBodyIndex :type Integer) (bFromSweep :type Boolean) (SweepResult :type "HitResult Structure (by ref)"))
  (bind _returnvalue_x (`KismetMathLibrary.BreakVector` (`SceneComponent.K2_GetComponentLocation` (`self.Arrow_L`))))
  ;[1 1 1] 左右端传送
  (bind _as2dside_scroller_character (cast `/Game/2DSideScrollerBP/Blueprints/2DSideScrollerCharacter` OtherActor))
  (bind (_returnvalue_x_2 _returnvalue_y _returnvalue_z) (`KismetMathLibrary.BreakVector` (`self.K2_GetActorLocation` _as2dside_scroller_character)))
  (`self.K2_SetActorLocation` _as2dside_scroller_character (`KismetMathLibrary.MakeVector` _returnvalue_x _returnvalue_y _returnvalue_z) false true))

(event `self.Death_Col.OnComponentBeginOverlap`
  (params (OverlappedComponent :type "PrimitiveComponent Object Reference") (OtherActor :type "Actor Object Reference") (OtherComp :type "PrimitiveComponent Object Reference") (OtherBodyIndex :type Integer) (bFromSweep :type Boolean) (SweepResult :type "HitResult Structure (by ref)"))
  ;[1 1 1] 死亡判定
  (bind _as2dside_scroller_character (cast `/Game/2DSideScrollerBP/Blueprints/2DSideScrollerCharacter` OtherActor))
  (bind (_returnvalue_x _returnvalue_y _returnvalue_z) (`KismetMathLibrary.BreakVector` (`self.GetVelocity` _as2dside_scroller_character)))
  (if (not (> _returnvalue_z -4000.0))
    ;[1 1 1] 延时0.3s结束游戏
    (`KismetSystemLibrary.Delay` 0.3)
    (set `/Game/2DSideScrollerBP/Blueprints/2DSideScrollerCharacter.If Dead` true _as2dside_scroller_character)))

(fn `UserConstructionScript`
  (bind _childactor (`self.ChildActor`))
  (bind _childactor1 (`self.ChildActor1`))
  (bind _childactor_win (`self.ChildActor_Win`))
  (bind (_relativelocation_x _relativelocation_y _relativelocation_z) (`KismetMathLibrary.BreakVector` (`SceneComponent.RelativeLocation` _childactor_win)))
  (bind (_relativelocation_x_2 _relativelocation_y_2 _relativelocation_z_2) (`KismetMathLibrary.BreakVector` (`SceneComponent.RelativeLocation` _childactor)))
  (bind (_relativelocation_x_3 _relativelocation_y_3 _relativelocation_z_3) (`KismetMathLibrary.BreakVector` (`SceneComponent.RelativeLocation` _childactor1)))
  (`SceneComponent.K2_SetRelativeLocation` _childactor (`KismetMathLibrary.MakeVector` (`KismetMathLibrary.RandomFloatInRange` -950.0 950.0) _relativelocation_y_2 _relativelocation_z_2) false false)
  (`SceneComponent.K2_SetRelativeLocation` _childactor1 (`KismetMathLibrary.MakeVector` (`KismetMathLibrary.RandomFloatInRange` -950.0 950.0) _relativelocation_y_3 _relativelocation_z_3) false false)
  (`SceneComponent.K2_SetRelativeLocation` _childactor_win (`KismetMathLibrary.MakeVector` _relativelocation_x _relativelocation_y _relativelocation_z) false false))