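; Initial map segment of level 03 in a 2D side-scroller, randomizing child actor X positions on construction and spawning an ulcer area at BeginPlay.
; A one-shot trigger spawns one of two random next segments at NextMapLocation, chaining the map procedurally.
; Side triggers wrap the character horizontally to the opposite arrow.
; The death trigger flags the character dead after a short delay if it enters falling too fast.
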(event `self.ReceiveBeginPlay`
  (bind (_returnvalue_x _returnvalue_y _returnvalue_z) (`KismetMathLibrary.BreakVector` (`self.K2_GetActorLocation`)))
  (`|SpawnActorFromClass` "/Game/2DSideScrollerBP/Blueprints/BP_UlcerArea.BP_UlcerArea_C" (`KismetMathLibrary.MakeTransform` (`KismetMathLibrary.MakeVector` (`KismetMathLibrary.RandomFloatInRange` -700.0 700.0) 0.0 (+ _returnvalue_z (`KismetMathLibrary.RandomFloatInRange` 100.0 1800.0)))) "Undefined" "OverrideRootScale" null null))

(event `self.NextMapCollision1.OnComponentBeginOverlap`
  (params (OverlappedComponent :type "PrimitiveComponent Object Reference") (OtherActor :type "Actor Object Reference") (OtherComp :type "PrimitiveComponent Object Reference") (OtherBodyIndex :type Integer) (bFromSweep :type Boolean) (SweepResult :type "HitResult Structure (by ref)"))
  ;[1 1 1] 下一map随机生成
  (`/Engine/EditorBlueprintResources/StandardMacros.DoOnce` false
    (:`Completed`
      (cast `/Game/2DSideScrollerBP/Blueprints/2DSideScrollerCharacter` OtherActor)
      (`|SpawnActorFromClass` (`|GetArrayItem` (`self.RandomMapGenerate`) (`KismetMathLibrary.RandomIntegerInRange` 0 1)) (`SceneComponent.K2_GetComponentToWorld` (`self.NextMapLocation`)) "Undefined" "OverrideRootScale" null null)
      (`ActorComponent.K2_DestroyComponent` (`self.NextMapCollision1`)))))

(event `self.Left_TeleportCol.OnComponentBeginOverlap`
  (params (OverlappedComponent :type "PrimitiveComponent Object Reference") (OtherActor :type "Actor Object Reference") (OtherComp :type "PrimitiveComponent Object Reference") (OtherBodyIndex :type Integer) (bFromSweep :type Boolean) (SweepResult :type "HitResult Structure (by ref)"))
  (bind _returnvalue_x (`KismetMathLibrary.BreakVector` (`SceneComponent.K2_GetComponentLocation` (`self.Arrow_R`))))
  ;[1 1 1] 左右端传送
  (bind _as2dside_scroller_character (cast `/Game/2DSideScrollerBP/Blueprints/2DSideScrollerCharacter` OtherActor))
  (bind (_returnvalue_x_2 _returnvalue_y _returnvalue_z) (`KismetMathLibrary.BreakVector` (`self.K2_GetActorLocation` _as2dside_scroller_character)))
  (`self.K2_SetActorLocation` _as2dside_scroller_character (`KismetMathLibrary.MakeVector` _returnvalue_x _returnvalue_y _returnvalue_z) false true))

(event `self.Right_TeleportCol.OnComponentBeginOverlap`
  (params (OverlappedComponent :type "PrimitiveComponent Object Reference") (OtherActor :type "Actor Object Reference") (OtherComp :type "PrimitiveComponent Object Reference") (OtherBodyIndex :type Integer) (bFromSweep :type Boolean) (SweepResult :type "HitResult Structure (by ref)"))
  (bind _returnvalue_x (`KismetMathLibrary.BreakVector` (`SceneComponent.K2_GetComponentLocation` (`self.Arrow_L`))))
  ;[1 1 1] 左右端传送
  (bind _as2dside_scroller_character (cast `/Game/2DSideScrollerBP/Blueprints/2DSideScrollerCharacter` OtherActor))
  (bind (_returnvalue_x_2 _returnvalue_y _returnvalue_z) (`KismetMathLibrary.BreakVector` (`self.K2_GetActorLocation` _as2dside_scroller_character)))
  (`self.K2_SetActorLocation` _as2dside_scroller_character (`KismetMathLibrary.MakeVector` _returnvalue_x _returnvalue_y _returnvalue_z) false true))

(event `self.Death_Col.OnComponentBeginOverlap`
  (params (OverlappedComponent :type "PrimitiveComponent Object Reference") (OtherActor :type "Actor Object Reference") (OtherComp :type "PrimitiveComponent Object Reference") (OtherBodyIndex :type Integer) (bFromSweep :type Boolean) (SweepResult :type "HitResult Structure (by ref)"))
  ;[1 1 1] 死亡判定
  (bind _as2dside_scroller_character (cast `/Game/2DSideScrollerBP/Blueprints/2DSideScrollerCharacter` OtherActor))
  (bind (_returnvalue_x _returnvalue_y _returnvalue_z) (`KismetMathLibrary.BreakVector` (`self.GetVelocity` _as2dside_scroller_character)))
  (if (not (> _returnvalue_z -4000.0))
    ;[1 1 1] 延时0.3s结束游戏
    (`KismetSystemLibrary.Delay` 0.3)
    (set `/Game/2DSideScrollerBP/Blueprints/2DSideScrollerCharacter.If Dead` true _as2dside_scroller_character)))

(fn `UserConstructionScript`
  (bind _childactor (`self.ChildActor`))
  (bind _childactor7 (`self.ChildActor7`))
  (bind _childactor2 (`self.ChildActor2`))
  (bind _childactor6 (`self.ChildActor6`))
  (bind (_relativelocation_x _relativelocation_y _relativelocation_z) (`KismetMathLibrary.BreakVector` (`SceneComponent.RelativeLocation` _childactor7)))
  (bind (_relativelocation_x_2 _relativelocation_y_2 _relativelocation_z_2) (`KismetMathLibrary.BreakVector` (`SceneComponent.RelativeLocation` _childactor6)))
  (bind (_relativelocation_x_3 _relativelocation_y_3 _relativelocation_z_3) (`KismetMathLibrary.BreakVector` (`SceneComponent.RelativeLocation` _childactor)))
  (bind (_relativelocation_x_4 _relativelocation_y_4 _relativelocation_z_4) (`KismetMathLibrary.BreakVector` (`SceneComponent.RelativeLocation` _childactor2)))
  (`SceneComponent.K2_SetRelativeLocation` _childactor (`KismetMathLibrary.MakeVector` (`KismetMathLibrary.RandomFloatInRange` 350.0 750.0) _relativelocation_y_3 _relativelocation_z_3) false false)
  (`SceneComponent.K2_SetRelativeLocation` _childactor2 (`KismetMathLibrary.MakeVector` (`KismetMathLibrary.RandomFloatInRange` 550.0 950.0) _relativelocation_y_4 _relativelocation_z_4) false false)
  (`SceneComponent.K2_SetRelativeLocation` _childactor7 (`KismetMathLibrary.MakeVector` (`KismetMathLibrary.SelectFloat` (`KismetMathLibrary.RandomFloatInRange` -700.0 -400.0) (`KismetMathLibrary.RandomFloatInRange` 450.0 650.0) (`KismetMathLibrary.RandomBool`)) _relativelocation_y _relativelocation_z) false false)
  (`SceneComponent.K2_SetRelativeLocation` _childactor6 (`KismetMathLibrary.MakeVector` (`KismetMathLibrary.RandomFloatInRange` -950.0 -750.0) _relativelocation_y_2 _relativelocation_z_2) false false))