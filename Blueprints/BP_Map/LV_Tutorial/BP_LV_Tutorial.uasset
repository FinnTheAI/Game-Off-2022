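; BP_LV_Tutorial is the tutorial map actor for a 2D side-scroller, handling screen-edge wrapping and fall death.
; Left and right triggers teleport the player to the opposite arrow's X, and set an overlapping enemy's SceneTransform to its negated X with zero Y/Z.
; The death trigger sets the player's IfDead after a short delay when falling fast enough.
; Random next-map and BP_UlcerArea spawning logic is present but disconnected.
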(event `self.ReceiveBeginPlay`)

(event `self.NextMapCollision1.OnComponentBeginOverlap`
  (params (OverlappedComponent :type "PrimitiveComponent Object Reference") (OtherActor :type "Actor Object Reference") (OtherComp :type "PrimitiveComponent Object Reference") (OtherBodyIndex :type Integer) (bFromSweep :type Boolean) (SweepResult :type "HitResult Structure (by ref)")))

(event `self.Left_TeleportCol.OnComponentBeginOverlap`
  (params (OverlappedComponent :type "PrimitiveComponent Object Reference") (OtherActor :type "Actor Object Reference") (OtherComp :type "PrimitiveComponent Object Reference") (OtherBodyIndex :type Integer) (bFromSweep :type Boolean) (SweepResult :type "HitResult Structure (by ref)"))
  (bind _returnvalue_x (`KismetMathLibrary.BreakVector` (`SceneComponent.K2_GetComponentLocation` (`self.Arrow_R`))))
  (`|ExecutionSequence`
    (:`then_0`
      ;[1 1 1] 左右端传送
      (bind _as2dside_scroller_character (cast `/Game/2DSideScrollerBP/Blueprints/2DSideScrollerCharacter` OtherActor))
      (bind (_returnvalue_x_2 _returnvalue_y _returnvalue_z) (`KismetMathLibrary.BreakVector` (`self.K2_GetActorLocation` _as2dside_scroller_character)))
      (`self.K2_SetActorLocation` _as2dside_scroller_character (`KismetMathLibrary.MakeVector` _returnvalue_x _returnvalue_y _returnvalue_z) false true))
    (:`then_1`
      ;[1 1 1] Comment
      (bind _asbp_enemy (cast `/Game/2DSideScrollerBP/Blueprints/BP_Enemy` OtherActor))
      (bind _scene_transform_location (`KismetMathLibrary.BreakTransform` (`/Game/2DSideScrollerBP/Blueprints/BP_Enemy.Scene Transform` _asbp_enemy)))
      (set `/Game/2DSideScrollerBP/Blueprints/BP_Enemy.Scene Transform` (`KismetMathLibrary.MakeTransform` (* _scene_transform_location (-1.0 0.0 0.0))) _asbp_enemy))))

(event `self.Right_TeleportCol.OnComponentBeginOverlap`
  (params (OverlappedComponent :type "PrimitiveComponent Object Reference") (OtherActor :type "Actor Object Reference") (OtherComp :type "PrimitiveComponent Object Reference") (OtherBodyIndex :type Integer) (bFromSweep :type Boolean) (SweepResult :type "HitResult Structure (by ref)"))
  (bind _returnvalue_x (`KismetMathLibrary.BreakVector` (`SceneComponent.K2_GetComponentLocation` (`self.Arrow_L`))))
  (`|ExecutionSequence`
    (:`then_0`
      ;[1 1 1] 左右端传送
      (bind _as2dside_scroller_character (cast `/Game/2DSideScrollerBP/Blueprints/2DSideScrollerCharacter` OtherActor))
      (bind (_returnvalue_x_2 _returnvalue_y _returnvalue_z) (`KismetMathLibrary.BreakVector` (`self.K2_GetActorLocation` _as2dside_scroller_character)))
      (`self.K2_SetActorLocation` _as2dside_scroller_character (`KismetMathLibrary.MakeVector` _returnvalue_x _returnvalue_y _returnvalue_z) false true))
    (:`then_1`
      ;[1 1 1] Comment
      (bind _asbp_enemy (cast `/Game/2DSideScrollerBP/Blueprints/BP_Enemy` OtherActor))
      (bind _scene_transform_location (`KismetMathLibrary.BreakTransform` (`/Game/2DSideScrollerBP/Blueprints/BP_Enemy.Scene Transform` _asbp_enemy)))
      (set `/Game/2DSideScrollerBP/Blueprints/BP_Enemy.Scene Transform` (`KismetMathLibrary.MakeTransform` (* _scene_transform_location (-1.0 0.0 0.0))) _asbp_enemy))))

(event `self.Death_Col.OnComponentBeginOverlap`
  (params (OverlappedComponent :type "PrimitiveComponent Object Reference") (OtherActor :type "Actor Object Reference") (OtherComp :type "PrimitiveComponent Object Reference") (OtherBodyIndex :type Integer) (bFromSweep :type Boolean) (SweepResult :type "HitResult Structure (by ref)"))
  ;[1 1 1] 死亡判定
  (bind _as2dside_scroller_character (cast `/Game/2DSideScrollerBP/Blueprints/2DSideScrollerCharacter` OtherActor))
  (bind (_returnvalue_x _returnvalue_y _returnvalue_z) (`KismetMathLibrary.BreakVector` (`self.GetVelocity` _as2dside_scroller_character)))
  (if (not (> _returnvalue_z -4000.0))
    ;[1 1 1] 延时0.3s结束游戏
    (`KismetSystemLibrary.Delay` 0.3)
    (set `/Game/2DSideScrollerBP/Blueprints/2DSideScrollerCharacter.If Dead` true _as2dside_scroller_character)))

(fn `UserConstructionScript`)