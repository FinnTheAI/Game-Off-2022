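; BP_Enemy_Bullet is an enemy projectile that flags itself dead on overlapping the 2DSideScrollerCharacter.
; BeginPlay destroys it if the game instance's IfInUI is set, otherwise activates its spit effect.
; Tick runs at a fixed interval, moving the bullet by a stored local transform outside UI, without delta-time scaling.
; Once dead, Tick disables collision, swaps Bullet01 for Bullet02 through short delays, then destroys the actor.
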(event `self.ReceiveBeginPlay`
  (`|ExecutionSequence`
    (:`then_0`
      ;[1 1 1] Comment
      (bind _asbp_game_instance (cast `/Game/2DSideScrollerBP/Blueprints/BP_Core/BP_GameInstance` (`GameplayStatics.GetGameInstance`)))
      (set `self.As BP Game Instance` _asbp_game_instance))
    (:`then_1`
      (if (`/Game/2DSideScrollerBP/Blueprints/BP_Core/BP_GameInstance.If in UI` (`self.As BP Game Instance`))
        (`ActorComponent.SetActive` (`self.吐子弹`) false false)
        (`ActorComponent.SetActive` (`self.BulletDestroy`) false false)
        (`self.K2_DestroyActor`)
        (else
          (`ActorComponent.SetActive` (`self.吐子弹`) true false)
          (`ActorComponent.SetActive` (`self.BulletDestroy`) false true))))
    (:`then_2`
      (`self.SetActorTickInterval` 0.02))))

(event `self.ReceiveTick`
  (params (DeltaSeconds :type "Float (single-precision)"))
  (set `self.Delta Seconds` DeltaSeconds)
  (if (not (`/Game/2DSideScrollerBP/Blueprints/BP_Core/BP_GameInstance.If in UI` (`self.As BP Game Instance`)))
    ;[1 1 1] 子弹位移
    (`SceneComponent.K2_AddLocalTransform` (`self.Bullet`) (`self.Bullet Transform Temp`) false false)
    ;[1 1 1] 敌人死亡判定
    (if (`self.Is Dead`)
      (`self.SetActorEnableCollision` false)
      (`SceneComponent.SetVisibility` (`self.Bullet_01`) false false)
      (`KismetSystemLibrary.Delay` 0.1)
      (`SceneComponent.SetVisibility` (`self.Bullet_02`) true false)
      (`KismetSystemLibrary.Delay` 0.25)
      (`self.K2_DestroyActor`))))

(event `self.Capsule.OnComponentBeginOverlap`
  (params (OverlappedComponent :type "PrimitiveComponent Object Reference") (OtherActor :type "Actor Object Reference") (OtherComp :type "PrimitiveComponent Object Reference") (OtherBodyIndex :type Integer) (bFromSweep :type Boolean) (SweepResult :type "HitResult Structure (by ref)"))
  (cast `/Game/2DSideScrollerBP/Blueprints/2DSideScrollerCharacter` OtherActor)
  (set `self.Is Dead` true))

(fn `UserConstructionScript`)